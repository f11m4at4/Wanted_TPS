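; Third-person shooter player Blueprint that drives the on-screen health and damage UI.
; BeginPlay creates the main HUD widget and adds it to the viewport.
; The PlayerDamage component's OnUpdateHealth event passes its current Hp to that HUD when the player is hit.
; ShowDamageUI lazily creates the damage widget on first use, then reuses it to display damage feedback.
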(event OnUpdateHealth(playerDamage)
  ;[0.15 0.15 0.15 0.5] 피격시 UI 갱신처리
  (bind _asplayer_damage (Utilities|Casting|CastToPlayerDamage (Variables|Default|GetplayerDamage)))
  (Default|UpdateHealth (Variables|Default|GetMainUI) (Variables|/Script/TPS.PlayerDamage|Gethp _asplayer_damage)))

(event EventShowDamageUI
  (Utilities|IsValid (Variables|Default|GetDamageUI)
    (:Is%20Valid
      (Default|ShowDamageUI (Variables|Default|GetDamageUI)))
    (:Is%20Not%20Valid
      (bind _returnvalue (UserInterface|CreateWidget "/Game/Blueprints/WBP_DamageUI.WBP_DamageUI_C"))
      (bind _output_get (Variables|Default|SetDamageUI _returnvalue))
      (UserInterface|Viewport|AddtoViewport _output_get 0)
      (Default|ShowDamageUI _output_get))))

(event EventBeginPlay
  (bind _returnvalue (UserInterface|CreateWidget "/Game/Blueprints/WBP_MainUI.WBP_MainUI_C"))
  (bind _output_get (Variables|Default|SetMainUI _returnvalue))
  (UserInterface|Viewport|AddtoViewport _output_get 0))

(fn ConstructionScript)